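; Base follow camera for a cowboy player that switches between Searching, Hunted and Hunter modes.
; Each tick it interpolates toward a mode-dependent target at the player's height, using per-mode offset and lag from CameraMetrics.
; A per-tick EQS query finds nearby foes, switching Searching to Hunted and centering both combat modes on the player-and-foe average.
; Armed status events from the cowboy enter or exit Hunter mode.
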(event Custom|Armed%20Status%20Camera%20Response
  (params (Is%20Armed :type Boolean))
  ;[1 1 1] Enter/Exit Hunter mode
  (Variables|Default|SetCurrent%20Mode (select Is%20Armed "NewEnumerator2" "NewEnumerator0")))

(event EventTick
  (params (DeltaSeconds :type Float%20%28single-precision%29))
  (bind _returnvalue (Game|GetInstigator))
  (bind _returnvalue_2 (Game|GetInstigator))
  (bind _returnvalue_3 (Game|GetInstigator))
  (bind _camera_metrics (Variables|Default|GetCamera%20Metrics))
  (bind _current_mode (Variables|Default|GetCurrent%20Mode))
  (bind _current_mode_2 (Variables|Default|GetCurrent%20Mode))
  (bind _hunted_target_location (Variables|Default|GetHunted%20Target%20Location))
  (bind _value (Utilities|Map|Find _camera_metrics _current_mode_2))
  (bind _returnvalue_4 (Transformation|GetActorLocation _returnvalue))
  (bind _returnvalue_5 (Utilities|Select :Index _current_mode :NewEnumerator0 _returnvalue_4 :NewEnumerator1 _hunted_target_location :NewEnumerator2 _hunted_target_location))
  (bind (_x _y) (Math|Vector|BreakVector _returnvalue_5))
  (Utilities|FlowControl|Sequence
    (:then_0
      ;[1 1 1] Camera Following
      (Utilities|IsValid _returnvalue
        (:Is%20Valid
          (Transformation|SetActorLocation (Math|Interpolation|VInterpTo (Transformation|GetActorLocation) (+ (Math|Vector|SelectVector (Math|Vector|MakeVector _x _y (.Z (Math|Vector|BreakVector (Transformation|GetActorLocation _returnvalue_3)))) (CallFunction|FindPlayerCenter) (Utilities|IsValid _returnvalue_3)) (.cameraoffset _value)) (Utilities|Time|GetWorldDeltaSeconds) (.cameralag _value)) false false))))
    (:then_1
      ;[1 1 1] Run Query to find nearby foes
      (Utilities|IsValid _returnvalue_2
        (:Is%20Valid
          (bind _returnvalue_6 (AI|EQS|RunEQSQuery "/Game/Blueprints/Camera/EQS_CameraEnemyDetection.EQS_CameraEnemyDetection" _returnvalue_2 "AllMatching" "/Script/AIModule.EnvQueryInstanceBlueprintWrapper"))
          (EventDispatchers|BindEventtoOnQueryFinishedEvent _returnvalue_6 (EventDispatchers|CreateEvent :!event DetermineHuntedCameraLocation)))))))

(event EventBeginPlay
  (bind _asbp_cowboy_base (Utilities|Casting|CastToBP_Cowboy_Base (Game|GetInstigator)))
  ;[1 1 1] Enter/Exit Hunter mode
  (EventDispatchers|BindEventtoArmedStatusUpdated _asbp_cowboy_base (EventDispatchers|CreateEvent :!event Custom|Armed%20Status%20Camera%20Response)))

(fn ConstructionScript
  (Transformation|SetActorLocation (.cameraoffset (.Value (Utilities|Map|Find (Variables|Default|GetCamera%20Metrics) (Variables|Default|GetCurrent%20Mode)))) false true))

(fn DetermineHuntedCameraLocation
  (params (EQS%20Query :type Env%20Query%20Instance%20Blueprint%20Wrapper%20Object%20Reference) (Query%20Status :type EEnvQueryStatus%20Enum :default "Processing"))
  (bind _returnvalue (Game|GetInstigator))
  (bind _resultactors (AI|EQS|GetQueryResultsasActors EQS%20Query))
  (bind _output_get (LocalVariables|SetSpotted%20Foes _resultactors))
  (if (Utilities|Array|ContainsItem _output_get _returnvalue)
    _
    (else
      (Utilities|Array|Add _output_get _returnvalue)))
  (switch Utilities|FlowControl|Switch|SwitchonE_CameraMode (Variables|Default|GetCurrent%20Mode)
    (:NewEnumerator0
      (if (> (Utilities|Array|Length (LocalVariables|GetSpotted%20Foes)) 1) :!label _label
        (Variables|Default|SetCurrent%20Mode "NewEnumerator1")
        (else
          (Variables|Default|SetCurrent%20Mode "NewEnumerator0"))))
    (:NewEnumerator1
      (goto _label))
    (:NewEnumerator2
      _))
  (bind _returnvalue_2 (Class|GameplayStatics|GetActorArrayAverageLocation (LocalVariables|GetSpotted%20Foes)))
  (Variables|Default|SetHunted%20Target%20Location _returnvalue_2)
  (return))

(fn FindPlayerCenter
  (bind _outactors (Actor|GetAllActorsOfClass "/Game/Blueprints/Character/BP_Cowboy_Base.BP_Cowboy_Base_C"))
  (bind _returnvalue (Class|GameplayStatics|GetActorArrayAverageLocation _outactors))
  (return _returnvalue))