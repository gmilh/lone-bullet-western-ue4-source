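; Base bullet actor that deals a fixed amount of bullet-type damage to whatever it hits, other than its owner.
; On a hit it credits the damage to the owner and its instigator controller when the owner is valid, then destroys itself.
; The impact particle effect spawns from the Destroyed event, so it plays on any destruction, not just on hits.
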(event EventDestroyed
  (Effects|SpawnEmitteratLocation "/Game/VFX/PS_BulletImpact.PS_BulletImpact" (Transformation|GetActorLocation) (Transformation|GetActorRotation)))

(event Collision|EventHit
  (params (MyComp :type Primitive%20Component%20Object%20Reference) (Other :type Actor%20Object%20Reference) (OtherComp :type Primitive%20Component%20Object%20Reference) (bSelfMoved :type Boolean) (HitLocation :type Vector :default "0, 0, 0") (HitNormal :type Vector :default "0, 0, 0") (NormalImpulse :type Vector :default "0, 0, 0") (Hit :type Hit%20Result%20Structure%20%28by%20ref%29))
  (bind _returnvalue (Components|GetOwner))
  (if (!= (Components|GetOwner) Other)
    (Utilities|IsValid _returnvalue
      (:Is%20Valid
        (Game|Damage|ApplyDamage Other 8e+02 (Game|GetInstigatorController _returnvalue) _returnvalue "/Game/Blueprints/Bullet/BP_Damage_Bullet.BP_Damage_Bullet_C"))
      (:Is%20Not%20Valid
        (Game|Damage|ApplyDamage Other 8e+02 0 0 "/Game/Blueprints/Bullet/BP_Damage_Bullet.BP_Damage_Bullet_C")))
    (Actor|DestroyActor)))

(fn ConstructionScript)