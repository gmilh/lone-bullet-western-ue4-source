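; Base breakable object that swaps itself for a broken version and can drop a bullet pickup.
; Bullet damage breaks it instantly; other damage costs one hit point per hit, with a hit sequence and effect, gated by a DoOnce until EnableHit resets it.
; Breaking forwards the damage to the spawned replacement and reads, then increments, the instigating pawn's luck, which sets the pickup chance rolled on Destroyed.
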(event Custom|Enable%20Hit
  (Utilities|FlowControl|DoOnce false) ; enters at Reset
)

(event EventDestroyed
  (if (Math|Random|RandomBoolwithWeight (Variables|Default|GetBullet%20Spawning%20Chance))
    (Game|SpawnActorfromClass "/Game/Blueprints/Bullet/BP_BulletPickup_Base.BP_BulletPickup_Base_C" (Transformation|GetActorTransform) "Undefined" 0 0)))

(event Game|Damage|EventAnyDamage
  (params (Damage :type Float%20%28single-precision%29) (DamageType :type Damage%20Type%20Object%20Reference) (InstigatedBy :type Controller%20Object%20Reference) (DamageCauser :type Actor%20Object%20Reference))
  (bind _returnvalue (Pawn|GetControlledPawn InstigatedBy))
  (Audio|PlaySoundatLocation (Variables|Default|GetDamaged%20Sound) (Transformation|GetActorLocation) "0, 0, 0" 1.0 1.0 0.0 "/Game/Audio/SA_VFX_Base.SA_VFX_Base" 0 0)
  (Utilities|Casting|CastToBP_Damage_Bullet DamageType
    (:then
      (bind _returnvalue_2 (Game|SpawnActorfromClass (Variables|Default|GetBroken%20Equivalent) (Transformation|GetActorTransform) "AlwaysSpawn" 0 0 :!label _label))
      (Game|Damage|ApplyDamage _returnvalue_2 Damage InstigatedBy DamageCauser (Utilities|GetClass DamageType))
      (Utilities|IsValid _returnvalue
        (:Is%20Valid
          (bind _luck (Class|BPIPickingUpBullet|GetLuck(Message) _returnvalue))
          (Variables|Default|SetBullet%20Spawning%20Chance _luck)
          (Class|BPIPickingUpBullet|IncrementLuck(Message) _returnvalue)
          (Actor|DestroyActor))
        (:Is%20Not%20Valid
          (Actor|DestroyActor))))
    (:CastFailed
      (Utilities|FlowControl|DoOnce false
        (:Completed
          (bind _result (Math|Integer|DecrementInt (Variables|Default|GetHit%20Points))
            (:%20%20
              (if (<= _result 0)
                (goto _label)
                (else
                  (Sequencer|Player|Play (Variables|/Script/ActorSequence.ActorSequenceComponent|GetSequencePlayer (Variables|Default|GetHit)) :!class /Script/MovieScene.MovieSceneSequencePlayer)
                  (Components|Activation|Activate (Variables|Default|GetHit%20Effect) false)
                  (Utilities|FlowControl|DoOnce false
                    (:Completed
                      (EventDispatchers|BindEventtoOnFinished (Variables|/Script/ActorSequence.ActorSequenceComponent|GetSequencePlayer (Variables|Default|GetHit)) (EventDispatchers|CreateEvent :!event Custom|Enable%20Hit)))))))))))))

(event EventSetBulletSpawningChance
  (params (Chance :type Float%20%28single-precision%29))
  (Variables|Default|SetBullet%20Spawning%20Chance Chance))

(fn ConstructionScript)