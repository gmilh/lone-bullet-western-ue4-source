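; BP_SlowMotionArea is a temporary area actor that applies its own CustomTimeDilation to actors inside it.
; BeginPlay dilates current overlaps, then opens a gate so later entrants are also dilated and tracked.
; After a delay counted in frames, it closes the gate, resets every valid tracked actor to normal time and destroys itself.
; Actors leaving the area stay dilated until then.
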(event OnComponentBeginOverlap(Area)
  (params (OverlappedComponent :type Primitive%20Component%20Object%20Reference) (OtherActor :type Actor%20Object%20Reference) (OtherComp :type Primitive%20Component%20Object%20Reference) (OtherBodyIndex :type Integer) (bFromSweep :type Boolean) (SweepResult :type Hit%20Result%20Structure%20%28by%20ref%29))
  (Utilities|FlowControl|Gate true
    (:Exit
      (Variables|/Script/Engine.Actor|SetCustomTimeDilation OtherActor (Variables|Default|GetCustom%20Time%20Dilation))
      (Utilities|Array|Add (Variables|Default|GetAffected%20Actors) OtherActor))))

(event EventBeginPlay
  (bind _output_get (Variables|Default|SetAffected%20Actors (Collision|GetOverlappingActors (Variables|Default|GetArea) "/Script/Engine.Actor" :!class /Script/Engine.PrimitiveComponent)))
  (for _array_element _output_get
    (Variables|/Script/Engine.Actor|SetCustomTimeDilation _array_element (Variables|Default|GetCustom%20Time%20Dilation)))
  (Utilities|FlowControl|Sequence
    (:then_0
      (Class|LowEntryExtendedStandardLibrary|DelayFrames (Variables|Default|GetEffect%20Duration%20%28Frames%29))
      (Utilities|FlowControl|Sequence
        (:then_0
          (Utilities|FlowControl|Gate true) ; enters at Close
        )
        (:then_1
          (for _array_element_2 (Variables|Default|GetAffected%20Actors)
            (Utilities|IsValid _array_element_2
              (:Is%20Valid
                (Variables|/Script/Engine.Actor|SetCustomTimeDilation _array_element_2 1.0))))
          (Actor|DestroyActor))))
    (:then_1
      (Utilities|FlowControl|Gate true) ; enters at Open
    )))

(fn ConstructionScript)