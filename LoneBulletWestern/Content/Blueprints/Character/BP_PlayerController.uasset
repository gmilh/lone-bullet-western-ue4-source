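; Player controller that links the possessed pawn to a game-mode-defined camera, the HUD and input-device detection.
; GetCamera lazily spawns and caches the camera class and angle supplied by the GameMode, and possession sets its Instigator and attaches the audio listener to the pawn.
; Any key press records gamepad use and informs the HUD, Pause toggles its paused message, and unpossessing switches the HUD enemy counter widget.
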(event EventSetMouseCursorEnabled
  (params (Enabled :type Boolean))
  (Variables|Default|SetbShowMouseCursor Enabled))

(event EventBeginPlay)

(event EventPossess
  (params (PossessedPawn :type Pawn%20Object%20Reference))
  (Variables|/Script/Engine.Actor|SetInstigator (CallFunction|GetCamera) PossessedPawn)
  (Class|PlayerController|SetAudioListenerOverride (Variables|/Script/Engine.Actor|GetRootComponent PossessedPawn) "0, 0, 0" "0, 0, 0"))

(event EventUnPossess
  (params (UnpossessedPawn :type Pawn%20Object%20Reference))
  (Variables|/Script/Engine.Actor|SetInstigator (CallFunction|GetCamera) 0)
  (bind _asbp_hud (Utilities|Casting|CastToBP_HUD (HUD|GetHUD)))
  (Class|WidgetSwitcher|SetActiveWidgetIndex (Variables|/Game/Blueprints/UI/WBP_SurvivorsCounter.WBP_SurvivorsCounter_C|GetWidgetSwitcher_80 (Variables|/Game/Blueprints/UI/BP_HUD.BP_HUD_C|GetEnemy%20Counter _asbp_hud)) 1))

(event Input|ActionEvents|InputActionPause
  (params (Key :type Key%20Structure))
  (:Pressed
    (Class|BPIUserInterface|TogglePaused(Message) (HUD|GetHUD))))

(event Input|KeyboardEvents|AnyKey
  (params (Key :type Key%20Structure))
  (:Pressed
    (Variables|Default|SetUsing%20Gamepad (Class|KismetInputLibrary|KeyIsGamepadKey Key))
    (Class|BPIUserInterface|DeclareInputDeviceType(Message) (HUD|GetHUD) (Variables|Default|GetUsing%20Gamepad))))

(fn ConstructionScript)

(fn GetCamera
  (bind _player_camera (Variables|Default|GetPlayer%20Camera)
    (:then
      (return _player_camera))
    (:else
      (bind (_camera_class _camera_angle) (Class|BPIGameModeData|GetCameraClass(Message) (Game|GetGameMode)))
      (bind _returnvalue (Game|SpawnActorfromClass _camera_class (Math|Transform|MakeTransform "0, 0, 0" _camera_angle "1,1,1") "Undefined" 0 0))
      (bind _output_get (Variables|Default|SetPlayer%20Camera _returnvalue))
      (return _output_get))))

(fn GetInputDeviceType
  (return (Variables|Default|GetUsing%20Gamepad)))

(fn GetUnderCursorHit
  (bind (_hitresult _returnvalue) (Game|Player|GetHitResultUnderCursorbyChannel "TraceTypeQuery1" true))
  (return _hitresult _returnvalue))