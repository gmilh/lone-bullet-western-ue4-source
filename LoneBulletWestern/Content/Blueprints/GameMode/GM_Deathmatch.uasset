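; Deathmatch game mode that tracks registered duelists and controls the match's background music.
; Duelist declarations and deaths update a counter and fire events, ending the duel when one or fewer remain.
; Armed-status changes from cowboys trigger a scan of their bullets, using a gate to choose armed music if anyone has ammo, otherwise search music.
; A separate idle track plays while the game is paused.
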(event Custom|Background%20Music%20Shift%20Check
  (params (Is%20Armed :type Boolean))
  ;[1 1 1] Swap background track when someone is armed
  (bind _outactors (Actor|GetAllActorsOfClass "/Game/Blueprints/Character/BP_Cowboy_Base.BP_Cowboy_Base_C"))
  (Utilities|FlowControl|Sequence
    (:then_0
      (goto _label_2 Open))
    (:then_1
      (bind _array_element (Utilities|Array|ForEachLoopwithBreak _outactors :!label _label)
        (:LoopBody
          (if (> (Variables|/Game/Blueprints/Character/BP_Cowboy_Base.BP_Cowboy_Base_C|GetBullets _array_element) 0)
            (Utilities|FlowControl|Sequence
              (:then_0
                (CallFunction|ChangeMusicTrack true))
              (:then_1
                (goto _label_2 Close))
              (:then_2
                (goto _label Break)))))
        (:Completed
          (Utilities|FlowControl|Gate true :!label _label_2
            (:Exit
              (CallFunction|ChangeMusicTrack false))))))))

(event EventBeginPlay
  ;[1 1 1] Initialise Background Music
  (Audio|Components|Audio|Play (Variables|Default|GetGame%20Search) 0.0)
  (Utilities|FlowControl|Delay 0.2)
  ;[1 1 1] Swap background track when someone is armed
  (bind _outactors (Actor|GetAllActorsOfClass "/Game/Blueprints/Character/BP_Cowboy_Base.BP_Cowboy_Base_C"))
  (for _array_element _outactors
    (EventDispatchers|BindEventtoArmedStatusUpdated _array_element (EventDispatchers|CreateEvent :!event Custom|Background%20Music%20Shift%20Check))))

(event EventSetPaused
  (params (Paused :type Boolean))
  ;[1 1 1] Pause Menu Music
  (if Paused
    (Audio|Components|Audio|Play (Variables|Default|GetGame%20Idle) 2.0)
    (else
      (Audio|Components|Audio|Stop (Variables|Default|GetGame%20Idle)))))

(event EventDeclareDuelist
  (params (Player :type Player%20Controller%20Object%20Reference) (Name :type String))
  (bind _result (Math|Integer|IncrementInt (Variables|Default|GetDuelists%20Number))
    (:%20%20
      (Default|CallUpdatedDuelistsRegistered _result))))

(event EventDeclareDeath
  (params (Player :type Player%20Controller%20Object%20Reference) (Name :type String))
  (bind _result (Math|Integer|DecrementInt (Variables|Default|GetDuelists%20Number))
    (:%20%20
      (Default|CallDuelistDied _result Player Name)
      (if (<= (Variables|Default|GetDuelists%20Number) 1)
        (Default|CallDuelEnds)))))

(fn ConstructionScript
  (|CallParentFunction))

(fn ChangeMusicTrack
  (params (Is%20Anyone%20Armed :type Boolean))
  (if Is%20Anyone%20Armed
    (if (Audio|Components|Audio|IsPlaying (Variables|Default|GetGame%20Search))
      (Class|AudioComponent|SetPaused (Variables|Default|GetGame%20Search) true)
      (Audio|Components|Audio|Play (Variables|Default|GetGame%20Armed) 0.2))
    (elif (Audio|Components|Audio|IsPlaying (Variables|Default|GetGame%20Armed))
      (Class|AudioComponent|SetPaused (Variables|Default|GetGame%20Search) false)
      (Audio|Components|Audio|FadeOut (Variables|Default|GetGame%20Armed) 0.8 0.0 :!class /Script/Engine.AudioComponent))))

(fn GetDuelists
  (|CallParentFunction)
  (return (Variables|Default|GetDuelists%20Number)))