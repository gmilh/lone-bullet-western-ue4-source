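; GM_DM_Enclosed is a game mode, likely for an enclosed deathmatch, that keeps the level stocked with breakable objects.
; On BeginPlay it spawns an initial set of barrels at breakable spawner locations and starts a looping respawn timer.
; Each tick of the timer counts intact breakables and restores a tiered number, more when fewer remain, by shuffling broken objects and calling their restore-spawner message.
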(event EventBeginPlay
  (|CallParentFunction)
  (CallFunction|InitialSpawn)
  (Utilities|Time|SetTimerbyFunctionName self "Breakables Respawning" (Variables|Default|GetRespawning%20Interval) true))

(fn ConstructionScript
  (|CallParentFunction))

(fn BreakablesRespawning
  (bind _outactors (Actor|GetAllActorsOfClass "/Game/Blueprints/Bullet/BP_BreakableObject_Base.BP_BreakableObject_Base_C"))
  (LocalVariables|SetBreakable%20Objects _outactors)
  (Math|Integer|CompareInt (Utilities|Array|Length (LocalVariables|GetBreakable%20Objects)) 5
    (:>
      (Math|Integer|CompareInt (Utilities|Array|Length (LocalVariables|GetBreakable%20Objects)) 15 :!label _label
        (:>
          (Math|Integer|CompareInt (Utilities|Array|Length (LocalVariables|GetBreakable%20Objects)) 25 :!label _label_2
            (:<
              (CallFunction|RespawnNBreakables 5))))
        (:==
          (goto _label_2))
        (:<
          (CallFunction|RespawnNBreakables 10))))
    (:==
      (goto _label))
    (:<
      (CallFunction|RespawnNBreakables 20))))

(fn RespawnNBreakables
  (params (N :type Integer))
  (bind _outactors (Actor|GetAllActorsOfClass "/Game/Blueprints/Bullet/BP_BrokenObject_Base.BP_BrokenObject_Base_C"))
  (bind _output_get (LocalVariables|SetBroken%20Objects _outactors))
  (Utilities|Array|Shuffle _output_get)
  (for _index (range 1 N)
    (Class|BPIBulletSpawner|RestoreSpawner(Message) (Utilities|Array|Get(acopy) (LocalVariables|GetBroken%20Objects) _index))))

(fn InitialSpawn
  (bind _outactors (Actor|GetAllActorsOfClass "/Game/Blueprints/Bullet/BP_BreakableSpawner.BP_BreakableSpawner_C"))
  (LocalVariables|SetSpawn%20Points _outactors)
  (for _index (range 1 (Variables|Default|GetInitial%20Breakables%20Amount))
    (Game|SpawnActorfromClass "/Game/Blueprints/Bullet/BP_Barrel.BP_Barrel_C" (Transformation|GetActorTransform (Utilities|Array|Get(acopy) (LocalVariables|GetSpawn%20Points) _index)) "Undefined" 0 0)))