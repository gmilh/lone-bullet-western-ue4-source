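; Game instance base that persists music and SFX volume between sessions in the "AudioData" save slot.
; On Init it loads the slot and applies the stored volumes to the soundtrack and SFX sound classes, or creates a BP_SaveData_Base save from their current volumes.
; PerformVolumeDataSave writes the current sound class volumes into the cached save object through message calls and saves the slot.
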(event EventInit
  (bind _returnvalue (SaveGame|DoesSaveGameExist "AudioData"))
  (if _returnvalue
    (bind _returnvalue_2 (SaveGame|LoadGamefromSlot "AudioData"))
    (Variables|Default|SetLoaded%20Save _returnvalue_2)
    (bind _volume (Class|BPIVolumeData|GetMusicVolume(Message) (Variables|Default|GetLoaded%20Save)))
    (Class|LowEntryExtendedStandardLibrary|SoundClassSetVolume "/Game/Audio/SC_Soundtrack_Master.SC_Soundtrack_Master" _volume)
    (bind _volume_2 (Class|BPIVolumeData|GetSFXVolume(Message) (Variables|Default|GetLoaded%20Save)))
    (Class|LowEntryExtendedStandardLibrary|SoundClassSetVolume "/Engine/EngineSounds/SFX.SFX" _volume_2)
    (else
      (bind _returnvalue_3 (SaveGame|CreateSaveGameObject "/Game/Blueprints/Saving/BP_SaveData_Base.BP_SaveData_Base_C"))
      (bind _output_get (Variables|Default|SetLoaded%20Save _returnvalue_3))
      (SaveGame|SaveGametoSlot _output_get "AudioData")
      (CallFunction|PerformVolumeDataSave))))

(event EventPerformVolumeDataSave
  (Class|BPIVolumeData|SetMusicVolume(Message) (Variables|Default|GetLoaded%20Save) (Class|LowEntryExtendedStandardLibrary|SoundClassGetVolume "/Game/Audio/SC_Soundtrack_Master.SC_Soundtrack_Master"))
  (Class|BPIVolumeData|SetSFXVolume(Message) (Variables|Default|GetLoaded%20Save) (Class|LowEntryExtendedStandardLibrary|SoundClassGetVolume "/Engine/EngineSounds/SFX.SFX"))
  (SaveGame|SaveGametoSlot (Variables|Default|GetLoaded%20Save) "AudioData"))